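; BP_interior is an interior object that highlights its static mesh through custom depth rendering while it is focused.
; OnFocus_1 turns custom depth on, and a short retriggerable delay turns it off once focus calls stop arriving.
; The Box overlap events are empty, and the nodes that toggle player input alongside the highlight are disconnected.
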(event OnComponentBeginOverlap(Box)
  (params (OverlappedComponent :type Primitive%20Component%20Object%20Reference) (OtherActor :type Actor%20Object%20Reference) (OtherComp :type Primitive%20Component%20Object%20Reference) (OtherBodyIndex :type Integer) (bFromSweep :type Boolean) (SweepResult :type Hit%20Result%20Structure%20%28by%20ref%29)))

(event OnComponentEndOverlap(Box)
  (params (OverlappedComponent :type Primitive%20Component%20Object%20Reference) (OtherActor :type Actor%20Object%20Reference) (OtherComp :type Primitive%20Component%20Object%20Reference) (OtherBodyIndex :type Integer)))

(event Custom|OnFocus_1
  (CallFunction|BeginFocus)
  (Variables|Default|Settimer 0.1)
  (Utilities|FlowControl|RetriggerableDelay (Variables|Default|Gettimer))
  (CallFunction|EndFocus))

(fn ConstructionScript)

(fn BeginFocus
  (Rendering|SetRenderCustomDepth (Variables|Debug|GetStaticMeshComponent) true))

(fn EndFocus
  (Rendering|SetRenderCustomDepth (Variables|Debug|GetStaticMeshComponent) false))