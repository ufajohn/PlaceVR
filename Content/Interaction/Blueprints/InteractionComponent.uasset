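; Interaction component that detects the interactable in front of the player camera and forwards interact calls to it with the player's controller and pawn.
; A looping timer runs box traces, using a half-size single trace when several objects are hit.
; Actors implementing InteractInterface supply interactable meshes, hover text and highlight settings.
; The focused actor drives the HUD prompt and a custom-depth outline colored through a Material Parameter Collection.
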(event Custom|Setup
  (params (InteractionDistance :type Float%20%28single-precision%29) (InteractFocusDistance :type Float%20%28single-precision%29) (TimeBetweenCheckForInteract :type Float%20%28single-precision%29) (TraceSize :type Float%20%28single-precision%29) (Trace%20Types :type Array%20of%20EObjectTypeQuery%20Enums) (InteractionHud :type Interaction%20Hud%20Object%20Reference) (DebugType :type EDrawDebugTrace%20Enum))
  ;[1 1 1] Setup default variables
  (Utilities|FlowControl|Sequence
    (:then_0
      (Variables|Default|SetInteractionDistance InteractionDistance)
      (Variables|Default|SetInteractFocusDistance InteractFocusDistance)
      (Variables|Default|SetTraceSize TraceSize)
      (Variables|Default|SetTimeBetweenCheckForInteract TimeBetweenCheckForInteract)
      (Variables|Default|SetTrace%20Types Trace%20Types)
      (Variables|Default|SetInteractionHud InteractionHud)
      (Variables|Default|SetDebugType DebugType))
    (:then_1
      ;;[1 1 1] Setup timer
      (Utilities|Time|SetTimerbyFunctionName 0 "Trace" TimeBetweenCheckForInteract true))))

(fn Trace
  (bind _returnvalue (Game|GetPlayerCameraManager 0))
  (bind _returnvalue_2 (Transformation|GetActorLocation _returnvalue))
  ;[1 1 1] Set Start and End
  (LocalVariables|SetStart _returnvalue_2) ; Set start value for later use
  (LocalVariables|SetEnd (+ _returnvalue_2 (* (Transformation|GetActorForwardVector _returnvalue) (Variables|Default|GetInteractFocusDistance)))) ; Set end value for later use
  ;[1 1 1] Trace for interactable's
  (bind _outhits (Class|KismetSystemLibrary|BoxTraceMultiforObjects (LocalVariables|GetStart) (LocalVariables|GetEnd) (Math|Conversions|ToVector(Float) (Variables|Default|GetTraceSize)) "0, 0, 0" (Variables|Default|GetTrace%20Types) true 0 (Variables|Default|GetDebugType) true)) ; Get all interactables in range and view
  ;[1 1 1] Smallen trace if needed
  (if (> (Utilities|Array|Length _outhits) 1) ; If more than one interactable is found, smallen the trace and look for the one closest to the middle of the screen.
    (bind _outhit (Class|KismetSystemLibrary|BoxTraceSingleforObjects (LocalVariables|GetStart) (LocalVariables|GetEnd) (Math|Conversions|ToVector(Float) (/ (Variables|Default|GetTraceSize) 2.0)) "0, 0, 0" (Variables|Default|GetTrace%20Types) true 0 (Variables|Default|GetDebugType) true)))
  ;[1 1 1] hit something?
  (if (.bBlockingHit (Collision|BreakHitResult (select (> (Utilities|Array|Length _outhits) 1) _outhit (Utilities|Array|Get(acopy) _outhits)))) ; Is there a blocking hit?
    ;[1 1 1] Set HitActor
    (Variables|Default|SethitActor (.HitActor (Collision|BreakHitResult (select (> (Utilities|Array|Length _outhits) 1) _outhit (Utilities|Array|Get(acopy) _outhits)))))
    ;[1 1 1] Is different actor?
    (if (!= (.HitActor (Collision|BreakHitResult (select (> (Utilities|Array|Length _outhits) 1) _outhit (Utilities|Array|Get(acopy) _outhits)))) (Variables|Core|GetInteractActor))
      ;[1 1 1] Set Interface
      (bind _asinteract_interface (Utilities|Casting|CastToInteractInterface (Variables|Default|GethitActor)) ; Does actor have interactinterface?
        (:then
          (bind _output_get (Variables|Default|SetInterface (Utilities|ToObject(Interface) _asinteract_interface)))
          ;[1 1 1] Get data
          (bind (_interacthovertext _textcolor _bshowonscreen _blightup _highlightmeshes _highlightskeletals _outlinecolor _interact_meshes _interact_skeletals) (Class|InteractInterface|GetData(Message) _output_get)) ; Get data from the actor using the interface
          ;[1 1 1] Is hit mesh an interactable
          (bind _containsobject (CallFunction|IsInteractableMesh (.HitComponent (Collision|BreakHitResult (select (> (Utilities|Array|Length _outhits) 1) _outhit (Utilities|Array|Get(acopy) _outhits)))) _interact_meshes _interact_skeletals))
          ;[1 1 1] Hide old mesh
          (if _containsobject
            (CallFunction|HideOld)
            ;[1 1 1] Can change the interactable?
            (if (Variables|Default|GetbCanChange)
              ;[1 1 1] Set Interact Actor and close possibility to change
              (Variables|Core|SetInteractActor (Variables|Default|GethitActor))
              (Variables|Default|SetbCanChange false)
              (Utilities|FlowControl|Sequence
                (:then_0
                  ;[1 1 1] Text
                  (bind (_interacthovertext_2 _textcolor_2 _bshowonscreen_2) (Class|InteractInterface|GetData(Message) (Variables|Default|GetInterface)))
                  ;;[1 1 1] Want to be on screen?
                  (if _bshowonscreen_2 ; Does actor want to be shown on screen?
                    ;;[1 1 1] Set text in umg
                    (Default|Update (Variables|Default|GetInteractionHud) _textcolor_2 (Utilities|Text|ToText(String) _interacthovertext_2))
                    (else
                      ;;[1 1 1] Hide
                      (Default|Hide (Variables|Default|GetInteractionHud))
                      (CallFunction|HideOld))))
                (:then_1
                  ;[1 1 1] Set Render Depth
                  (bind (_interacthovertext_3 _textcolor_3 _bshowonscreen_3 _blightup_2 _highlightmeshes_2 _highlightskeletals_2 _outlinecolor_2) (Class|InteractInterface|GetData(Message) (Variables|Default|GetInterface)))
                  (if _blightup_2 ; Does actor want to be highlighted?
                    (Rendering|Material|SetVectorParameterValue "/Game/Interaction/Materials/Color.Color" "Color" _outlinecolor_2 :!class /Script/Engine.KismetMaterialLibrary)
                    (CallFunction|SetRenderDepth _highlightmeshes_2 _highlightskeletals_2 _highlightmeshes_2 _highlightskeletals_2)))))))
        (:CastFailed
          ;[1 1 1] Hide
          (Default|Hide (Variables|Default|GetInteractionHud) :!label _label) ; Hide if not in range/view
          (CallFunction|HideOld))))
    (else
      (goto _label))))

(fn HideOld
  ;[1 1 1] Cast to interface
  (bind _asinteract_interface (Utilities|Casting|CastToInteractInterface (Variables|Core|GetInteractActor)) ; Does actor have interactinterface?
    (:then
      ;[1 1 1] Get data
      (bind (_interacthovertext _textcolor _bshowonscreen _blightup _highlightmeshes _highlightskeletals) (Default|GetData _asinteract_interface))
      ;[1 1 1] remove render depth
      (for _array_element _highlightmeshes
        (Utilities|IsValid _array_element
          (:Is%20Valid
            (Rendering|SetRenderCustomDepth _array_element false))))
      (for _array_element_2 _highlightskeletals
        (Utilities|IsValid _array_element_2
          (:Is%20Valid
            (Rendering|SetRenderCustomDepth _array_element_2 false))))
      (Variables|Default|SetbCanChange true))
    (:CastFailed
      _))
  (Variables|Core|SetInteractActor 0)
  (return))

(fn Interact
  ;[1 1 1] Interact
  (Class|InteractInterface|InteractwithObject(Message) (Variables|Core|GetInteractActor) (Game|GetPlayerController 0) (Game|Player|GetPlayerPawn 0)))

(fn IsInteractableMesh
  (params (Object :type Object%20Object%20Reference) (TargetArray :type Array%20of%20Static%20Mesh%20Component%20Object%20References) (TargetArray2 :type Array%20of%20Skeletal%20Mesh%20Component%20Object%20References))
  ;[1 1 1] Force to false
  (LocalVariables|SetContains false)
  (for _array_element TargetArray
    (Utilities|IsValid _array_element
      (:Is%20Valid
        ;[1 1 1] Is hit mesh same as mesh in list
        (bind _asstatic_mesh_component (Utilities|Casting|CastToStaticMeshComponent Object))
        (if (== _asstatic_mesh_component _array_element)
          ;[1 1 1] Set true
          (LocalVariables|SetContains true)))))
  (for _array_element_2 TargetArray2
    ;[1 1 1] Is hit skeletal in list
    (Utilities|IsValid _array_element_2
      (:Is%20Valid
        (bind _asskeletal_mesh_component (Utilities|Casting|CastToSkeletalMeshComponent Object))
        (if (!= _asskeletal_mesh_component _array_element_2)
          (LocalVariables|SetContains true)))))
  ;[1 1 1] Return
  (return (LocalVariables|GetContains)))

(fn SetRenderDepth
  (params (TargetArray :type Array%20of%20Static%20Mesh%20Component%20Object%20References) (TargetArray2 :type Array%20of%20Skeletal%20Mesh%20Component%20Object%20References) (InputPin :type Array%20of%20Static%20Mesh%20Component%20Object%20References) (InputPin2 :type Array%20of%20Skeletal%20Mesh%20Component%20Object%20References))
  (Utilities|FlowControl|Sequence
    (:then_0
      ;[1 1 1] Set Render Depth
      (if (> (Utilities|Array|Length TargetArray2) 0)
        (for _array_element InputPin
          (Utilities|IsValid _array_element
            (:Is%20Valid
              (Rendering|SetRenderCustomDepth _array_element true))))))
    (:then_1
      ;[1 1 1] Set Render Depth
      (if (> (Utilities|Array|Length TargetArray) 0)
        (for _array_element_2 InputPin2
          (Utilities|IsValid _array_element_2
            (:Is%20Valid
              (Rendering|SetRenderCustomDepth _array_element_2 true))))))
    (:then_2
      ;[1 1 1] Return
      (return))))

(fn GetData
  (return "" "" false false (Utilities|Array|MakeArray 0) (Utilities|Array|MakeArray 0) "" (Utilities|Array|MakeArray 0) (Utilities|Array|MakeArray 0)))